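; BP_LimitWAll is a map limit wall actor that can be switched on and off as a barrier.
; It exposes two events, LimitWall_On and LimitWall_Off, which set collision (QueryAndPhysics or NoCollision) and visibility on four static mesh components together.
; BeginPlay and the construction script are empty, so the wall's state changes only when one of these events is called.
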(event `self.ReceiveBeginPlay`)

(event `LimitWall_Off`
  (`PrimitiveComponent.SetCollisionEnabled` (`self.StaticMesh`) "NoCollision")
  (`PrimitiveComponent.SetCollisionEnabled` (`self.StaticMesh1`) "NoCollision")
  (`PrimitiveComponent.SetCollisionEnabled` (`self.StaticMesh2`) "NoCollision")
  (`PrimitiveComponent.SetCollisionEnabled` (`self.StaticMesh3`) "NoCollision")
  (`SceneComponent.SetVisibility` (`self.StaticMesh`) false false)
  (`SceneComponent.SetVisibility` (`self.StaticMesh1`) false false)
  (`SceneComponent.SetVisibility` (`self.StaticMesh2`) false false)
  (`SceneComponent.SetVisibility` (`self.StaticMesh3`) false false))

(event `LimitWall_On`
  (`PrimitiveComponent.SetCollisionEnabled` (`self.StaticMesh`) "QueryAndPhysics")
  (`PrimitiveComponent.SetCollisionEnabled` (`self.StaticMesh1`) "QueryAndPhysics")
  (`PrimitiveComponent.SetCollisionEnabled` (`self.StaticMesh2`) "QueryAndPhysics")
  (`PrimitiveComponent.SetCollisionEnabled` (`self.StaticMesh3`) "QueryAndPhysics")
  (`SceneComponent.SetVisibility` (`self.StaticMesh`) true false)
  (`SceneComponent.SetVisibility` (`self.StaticMesh1`) true false)
  (`SceneComponent.SetVisibility` (`self.StaticMesh2`) true false)
  (`SceneComponent.SetVisibility` (`self.StaticMesh3`) true false))

(fn `UserConstructionScript`)