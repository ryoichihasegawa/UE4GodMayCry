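; BP_Zenyatta_Bullets_Tall is a player projectile that pierces enemies and destroys itself after three seconds or on overlapping a Boss_Wall enemy.
; Box overlaps with Enemy-tagged actors play a wind sound and send damage through an event message, without hit reaction.
; Tick re-enables Box collision and a Delay periodically switches it off, so lingering overlaps can hit again.
; The Horming event turns on ProjectileMovement homing toward a component added to the given target.
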(event `self.ReceiveBeginPlay`
  (`KismetSystemLibrary.Delay` 3.0)
  (`self.K2_DestroyActor`))

(event `self.ReceiveTick`
  (params (DeltaSeconds :type "Float (single-precision)"))
  (`PrimitiveComponent.SetCollisionEnabled` (`self.Box`) "QueryAndPhysics")
  (`KismetSystemLibrary.Delay` 0.5)
  (`PrimitiveComponent.SetCollisionEnabled` (`self.Box`) "NoCollision")
  (`KismetSystemLibrary.Delay` 0.5))

(event `Horming`
  (params (InputObject :type "Actor Object Reference"))
  (bind _projectilemovement (`self.ProjectileMovement`))
  (`/Engine/EditorBlueprintResources/StandardMacros.IsValid` InputObject
    (:`Is Valid`
      (bind _returnvalue (`AddComponent|NODE_AddSceneComponent-0` :`self` InputObject))
      (set `ProjectileMovementComponent.HomingTargetComponent` _returnvalue _projectilemovement)
      (set `ProjectileMovementComponent.bIsHomingProjectile` true _projectilemovement)
      (set `ProjectileMovementComponent.HomingAccelerationMagnitude` 2000.0 _projectilemovement))))

(event `self.Box.OnComponentBeginOverlap`
  (params (OverlappedComponent :type "PrimitiveComponent Object Reference") (OtherActor :type "Actor Object Reference") (OtherComp :type "PrimitiveComponent Object Reference") (OtherBodyIndex :type Integer) (bFromSweep :type Boolean) (SweepResult :type "HitResult Structure (by ref)"))
  ;[1 1 1] 当たり判定
  (if (`self.ActorHasTag` OtherActor "Enemy")
    (if (`self.ActorHasTag` OtherActor "Boss_Wall")
      (`self.K2_DestroyActor`)
      (else
        (`GameplayStatics.PlaySound2D` "/Game/Player/Sound/Attack/Wind_Attack.Wind_Attack" 0.4 1.0 0.0 null null)
        (message `/Game/Share_Parameter/BPI/BPI_Damage.playerDamageToEnemyEvent` OtherActor null (make `/Game/Share_Parameter/Struct/ST_Damage_Value` 20.0))))))

(fn `UserConstructionScript`)