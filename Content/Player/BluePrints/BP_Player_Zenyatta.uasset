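; BP_Player_Zenyatta is a player character child Blueprint that configures the Zenyatta variant with the "Power" attack, cancel, damage and step montages plus an attack sound.
; BeginPlay runs an init event that calls parent BeginPlay, assigns those assets to inherited variables and caches the game instance, then sets its PlayerMode to 2.
; Tick, overlap and construction logic simply defer to the parent.
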(event `Zenyatta_Init`
  (set `self.Player_Parent` false)
  (`parent.ReceiveBeginPlay`)
  (set `self.NormalMotion_Fly` "/Game/Player/Animation/Attack/Power/AMM_AttackFly_Power.AMM_AttackFly_Power")
  (set `self.Special_Motion_Fly` "/Game/Player/Animation/Attack/Power/AMM_AttackFly_Power.AMM_AttackFly_Power")
  (set `self.NormalMotion` "/Game/Player/Animation/Attack/Power/AMM_Cancell_Attack_Power.AMM_Cancell_Attack_Power")
  (set `self.Special_Motion` "/Game/Player/Animation/Attack/Power/AMM_CancellAttack_Special_Power.AMM_CancellAttack_Special_Power")
  (set `self.DamageMotion` "/Game/Player/Animation/Motion/Power/AMM_Power_Damage.AMM_Power_Damage")
  (set `self.StepMotion` "/Game/Player/Animation/Motion/Power/AMM_Power_Step.AMM_Power_Step")
  (set `self.Attack_Normal` "/Game/Player/Animation/Attack/Power/AMM_AttackPower.AMM_AttackPower")
  (set `self.Normal_AttackFly` "/Game/Player/Animation/Attack/Power/AMM_AttackFly_Power.AMM_AttackFly_Power")
  (set `self.Player_Parent` true)
  (set `self.Attack_Sword_Sound` "/Game/Player/Sound/Power_Attack01.Power_Attack01")
  (`/Engine/EditorBlueprintResources/StandardMacros.DoOnce` false
    (:`Completed`
      (bind _asbpgi_game_sysytem_count (cast `/Game/Share_Parameter/BPGI_GameSysytemCount` (`GameplayStatics.GetGameInstance`)))
      (set `self.As BPGI Game Sysytem Count` _asbpgi_game_sysytem_count))))

(event `self.ReceiveBeginPlay`
  (`self.Zenyatta_Init`)
  (set `/Game/Share_Parameter/BPGI_GameSysytemCount.Player_Mode` 2 (`self.As BPGI Game Sysytem Count`)))

(event `self.ReceiveTick`
  (params (DeltaSeconds :type "Float (single-precision)"))
  (`parent.ReceiveTick` DeltaSeconds))

(event `self.ReceiveActorBeginOverlap`
  (params (OtherActor :type "Actor Object Reference"))
  (`parent.ReceiveActorBeginOverlap` OtherActor))

(fn `UserConstructionScript`
  (`parent.UserConstructionScript`))