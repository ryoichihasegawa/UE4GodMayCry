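; BP_EnemySlime is a slime enemy Blueprint that builds on a parent class, forwarding construction, BeginPlay, Tick and actor overlap to it.
; Its Jumping function calls EnemyJump, and Attack plays the attack montage, ignoring its SectionName input.
; The attack collision's overlap spawns a Niagara effect at the other actor's location, gated by an actor tag check left at None.
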(event `self.ReceiveBeginPlay`
  (`parent.ReceiveBeginPlay`))

(event `self.ReceiveActorBeginOverlap`
  (params (OtherActor :type "Actor Object Reference"))
  (`parent.ReceiveActorBeginOverlap` OtherActor))

(event `self.ReceiveTick`
  (params (DeltaSeconds :type "Float (single-precision)"))
  (`parent.ReceiveTick` DeltaSeconds))

(event `self.AttackCollsion.OnComponentBeginOverlap`
  (params (OverlappedComponent :type "PrimitiveComponent Object Reference") (OtherActor :type "Actor Object Reference") (OtherComp :type "PrimitiveComponent Object Reference") (OtherBodyIndex :type Integer) (bFromSweep :type Boolean) (SweepResult :type "HitResult Structure (by ref)"))
  (if (`self.ActorHasTag` OtherActor "None")
    (`NiagaraFunctionLibrary.SpawnSystemAtLocation` null (`self.K2_GetActorLocation` OtherActor))))

(fn `Attack`
  (params (SectionName :type Name))
  (returns (attackTime :type "Float (double-precision)"))
  (bind _returnvalue (`self.PlayAnimMontage` (`self.m_attackMontage`)))
  (return _returnvalue))

(fn `Jumping`
  (`self.enemyJump`))

(fn `UserConstructionScript`
  (`parent.UserConstructionScript`))