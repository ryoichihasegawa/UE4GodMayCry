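; Slime enemy Character Blueprint that moves by hopping.
; BeginPlay runs the parent logic, then sets the walk speed.
; Each Tick runs the parent Tick, then calls Jump while max walk speed is above zero and StopJumping otherwise.
; The overlap event is disabled, and the construction script only calls the parent.
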(event `self.ReceiveBeginPlay`
  (`parent.ReceiveBeginPlay`)
  (set `CharacterMovementComponent.MaxWalkSpeed` 300.0 (`self.CharacterMovement`)))

(event `self.ReceiveTick`
  (params (DeltaSeconds :type "Float (single-precision)"))
  (`parent.ReceiveTick` DeltaSeconds)
  (if (> (`CharacterMovementComponent.MaxWalkSpeed` (`self.CharacterMovement`)) 0.0)
    (`self.Jump`)
    (else
      (`self.StopJumping`))))

(fn `UserConstructionScript`
  (`parent.UserConstructionScript`))