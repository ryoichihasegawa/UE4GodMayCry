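; Base enemy Character providing combat actions and reactions to player hits.
; On damage, grounded enemies play a hit montage and are launched by the player's HitReaction type, while falling enemies briefly hang midair with zeroed gravity.
; Callable helpers cover forward movement, jumping, spinning, facing the player, toggling attack collision and playing randomly chosen attack montage sections.
; Query functions report flying or falling state, horizontal distance to the player and remaining health.
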(event `self.disableenemyDamageCollision`
  ;[0.9234 0.1284 1] コリジョン判定の切り替え
  (`PrimitiveComponent.SetCollisionEnabled` (`self.AttackCollsion`) "NoCollision"))

(event `self.enableEnemyDamageCollision`
  ;[0.9234 0.1284 1] コリジョン判定の切り替え
  (`PrimitiveComponent.SetCollisionEnabled` (`self.AttackCollsion`) "QueryAndPhysics"))

(event `self.ReceiveBeginPlay`
  ;[1 0 0] 初期化
  (`parent.ReceiveBeginPlay`)
  (bind _asbp_player_pawn (cast `/Game/Player/BluePrints/BP_PlayerPawn` (`GameplayStatics.GetPlayerPawn` 0)))
  (set `self.m_player` _asbp_player_pawn)
  (`self.disableEnemyDamageCollision`))

(event `self.ReceiveActorBeginOverlap`
  (params (OtherActor :type "Actor Object Reference"))
  (`parent.ReceiveActorBeginOverlap` OtherActor))

(event `self.ReceiveTick`
  (params (DeltaSeconds :type "Float (single-precision)"))
  (`parent.ReceiveTick` DeltaSeconds))

(event `Hit`
  (bind _m_player (`self.m_player`))
  (bind _playerforward (`/Game/Player/BluePrints/BP_PlayerPawn.PlayerForward` _m_player))
  ;[1 1 1] プレイヤーからダメージを受けた時のノックバックイベント
  (`|PlayMontage` (`self.Mesh`) (`self.m_hitDamage`)
    (:`then`
      (switch `int` (`/Game/Player/BluePrints/BP_PlayerPawn.Hit_Reaction` _m_player)
        (:`0`
          (`self.LaunchCharacter` (* (`SceneComponent.GetForwardVector` _playerforward) 500.0)))
        (:`1`
          (`self.LaunchCharacter` (0.0 0.0 700.0))
          (set `CharacterMovementComponent.GravityScale` 0.8 (`self.CharacterMovement`))
          (message `/Game/Player/BPI/BPI_AttackGate.Camera_SeekSkyAttack` (`self.m_player`)))
        (:`2`
          (`self.LaunchCharacter` (* (`SceneComponent.GetForwardVector` _playerforward) 1000.0)))))))

(event `/Game/Share_Parameter/BPI/BPI_Damage.playerDamageToEnemyEvent`
  (params (damageActor :type "Actor Object Reference") (damageParam :type "/Game/Share_Parameter/Struct/ST_Damage_Value Structure"))
  (if (`|EnumEquality` (`CharacterMovementComponent.MovementMode` (`self.CharacterMovement`)) "MOVE_Falling")
    (`self.FlyHit`)
    (else
      (`self.Hit`))))

(event `FlyHit`
  ;[1 1 1] 空中にいるときにヒットした時のイベント
  (message `/Game/Player/BPI/BPI_AttackGate.Camera_SeekSkyAttack` (`self.m_player`))
  (set `CharacterMovementComponent.GravityScale` 0.0 (`self.CharacterMovement`))
  (set `MovementComponent.Velocity` (0.0 0.0 0.0) (`self.CharacterMovement`))
  (`KismetSystemLibrary.Delay` 0.5)
  (set `CharacterMovementComponent.GravityScale` 0.7 (`self.CharacterMovement`)))

(event `/Game/Enemy/BPI/BPI_EnemyAction.frontMove`
  ;[1 1 1] 前方に進む
  (`self.K2_AddActorWorldOffset` (* (`SceneComponent.GetForwardVector` (`self.frontArrow`)) (`self.m_speedAccele`)) true))

(event `/Game/Enemy/BPI/BPI_EnemyAction.enemyJump`
  ;[1 1 1] ジャンプするカスタム関数
  (`self.Jump`))

(event `/Game/Enemy/BPI/BPI_EnemyAction.keepSpinning`
  (params (time :type "Float (single-precision)"))
  ;[1 1 1] 回転し続ける処理
  (`self.K2_AddActorLocalRotation` (`KismetMathLibrary.MakeRotator` 0.0 0.0 (* time (`self.m_spinRotateValue`)))))

(event `/Game/Enemy/BPI/BPI_EnemyAction.rotateToTarget`
  ;[1 1 1] エネミーがプレイヤーに向く処理
  (`self.K2_SetActorRotation` (`KismetMathLibrary.MakeRotator` 0.0 0.0 (.yaw (`KismetMathLibrary.RInterpTo` (`self.K2_GetActorRotation`) (`KismetMathLibrary.FindLookAtRotation` (`self.K2_GetActorLocation`) (`self.K2_GetActorLocation` (`self.m_player`))) 10.0 100.0))) true))

(fn `Attack`
  (params (SectionName :type Name))
  (returns (attackTime :type "Float (double-precision)"))
  (bind _returnvalue (`self.PlayAnimMontage` (`self.m_attackMontage`) 1.0 SectionName))
  (return _returnvalue))

(fn `attackSection`
  (returns (getSectionName :type Name))
  (bind _returnvalue (`KismetMathLibrary.RandomBoolWithWeight` (`self.randomRange`)))
  (if _returnvalue
    (set `self.m_sectionName` "attack01")
    (else
      (set `self.m_sectionName` "attack02")))
  (`KismetSystemLibrary.PrintString` (`KismetStringLibrary.Conv_BoolToString` _returnvalue))
  (return (`self.m_sectionName`)))

(fn `closeRange`
  (params (selfActor :type "Actor Object Reference"))
  (returns (m_rangeReturn :type "Float (double-precision)"))
  (return (`KismetMathLibrary.VSizeXY` (- (`self.K2_GetActorLocation` selfActor) (`self.K2_GetActorLocation` (`self.m_player`))))))

(fn `enemyFallingCheck`
  (returns (`isFalling?` :type Boolean))
  (return (`NavMovementComponent.IsFalling` (`self.CharacterMovement`))))

(fn `enemyFlyingCheck`
  (returns (`isFlying?` :type Boolean))
  (return (`NavMovementComponent.IsFlying` (`self.CharacterMovement`))))

(fn `isAlive`
  (returns (Param :type Boolean))
  (bind _enemy_hp (`self.enemy_hp`))
  (`KismetSystemLibrary.PrintString` (`KismetStringLibrary.Conv_DoubleToString` _enemy_hp) true true (struct :`G` 0.66 :`B` 1.0 :`A` 1.0) _enemy_hp)
  (return (> _enemy_hp 0.0)))

(fn `setwidget`
  (return))

(fn `UserConstructionScript`)